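; Out-of-bounds trigger volume that restarts the level if the player's bike stays inside it too long.
; Overlap by a non-AI bp_bike starts a countdown and shows the bike's OutOfBoundsUI, and leaving resets the timer and hides it.
; Tick runs the countdown, pushes whole seconds to that UI, and reopens the current level by name when time runs out.
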(event EventBeginPlay
  (CallFunction|ResetTimer))

(event Collision|EventActorBeginOverlap
  (params (OtherActor :type Actor%20Object%20Reference))
  (bind _asbp_bike (Utilities|Casting|CastTobp_bike OtherActor))
  (if (not (Variables|/Game/Blueprints/Bike_BP/bp_bike.bp_bike_C|GetisAI _asbp_bike))
    (Variables|Default|SetisOutOfBounds true)
    (CallFunction|ShowTimer)))

(event EventTick
  (params (DeltaSeconds :type Float%20%28single-precision%29))
  (CallFunction|RunTimer DeltaSeconds)
  (if (<= (Variables|Default|GetcoolDownTime) 0.0)
    (bind _returnvalue (Game|GetCurrentLevelName true))
    (Game|OpenLevel(byName) (Utilities|String|StringToName _returnvalue))))

(event Collision|EventActorEndOverlap
  (params (OtherActor :type Actor%20Object%20Reference))
  (bind _asbp_bike (Utilities|Casting|CastTobp_bike OtherActor))
  (if (not (Variables|/Game/Blueprints/Bike_BP/bp_bike.bp_bike_C|GetisAI _asbp_bike))
    (CallFunction|ResetTimer)
    (CallFunction|HideTimer)))

(fn ConstructionScript)

(fn RunTimer
  (params (Delta :type Float%20%28single-precision%29))
  (if (Variables|Default|GetisOutOfBounds)
    (Variables|Default|SetcoolDownTime (- (Variables|Default|GetcoolDownTime) Delta))
    (bind _asbp_bike (Utilities|Casting|CastTobp_bike (Game|Player|GetPlayerPawn 0)))
    (Widget|SetVisibility (Variables|/Game/Blueprints/Bike_BP/bp_bike.bp_bike_C|GetoutOfBoundsUI _asbp_bike) "Visible")
    (Variables|/Game/Widgets/OutOfBoundsTimer.OutOfBoundsTimer_C|Settime (Variables|/Game/Blueprints/Bike_BP/bp_bike.bp_bike_C|GetoutOfBoundsUI _asbp_bike) (+ (Math|Float|Truncate (Variables|Default|GetcoolDownTime)) 1))
    (return)))

(fn ResetTimer
  (Variables|Default|SetcoolDownTime (Variables|Default|GetmaxCoolDownTime))
  (Variables|Default|SetisOutOfBounds false)
  (bind _asvehicle_blueprint (Utilities|Casting|CastToVehicleBlueprint (Game|Player|GetPlayerPawn 0))))

(fn HideTimer
  (bind _asbp_bike (Utilities|Casting|CastTobp_bike (Game|Player|GetPlayerPawn 0)))
  (Widget|SetVisibility (Variables|/Game/Blueprints/Bike_BP/bp_bike.bp_bike_C|GetoutOfBoundsUI _asbp_bike) "Hidden")
  (return))

(fn ShowTimer
  (bind _asbp_bike (Utilities|Casting|CastTobp_bike (Game|Player|GetPlayerPawn 0)))
  (Widget|SetVisibility (Variables|/Game/Blueprints/Bike_BP/bp_bike.bp_bike_C|GetoutOfBoundsUI _asbp_bike) "Visible"))