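; Booster actor that launches the player's bike forward when the bike overlaps it.
; On overlap, it casts the other actor to bp_bike and applies one very large force to that bike's mesh.
; The force follows the normalized forward vector of the bike's base aim rotation, so the push goes where the rider aims rather than along the booster's orientation.
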(event EventBeginPlay)

(event Collision|EventActorBeginOverlap
  (params (OtherActor :type Actor%20Object%20Reference))
  (bind _asbp_bike (Utilities|Casting|CastTobp_bike OtherActor))
  (Physics|AddForce (Variables|/Script/PhysXVehicles.WheeledVehicle|GetMesh _asbp_bike) (* (Math|Vector|Normalize (Math|Vector|GetForwardVector (Pawn|GetBaseAimRotation _asbp_bike))) 2e+08) "None" false))

(event EventTick
  (params (DeltaSeconds :type Float%20%28single-precision%29)))

(fn ConstructionScript)