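; A respawning pickup that gives an overlapping bp_bike a random powerup: Boost, Throwable or MegaTakeDown.
; On BeginPlay it picks a type and matching food-themed mesh, with Throwable randomly using one of two meshes.
; Overlap copies the type string to the bike, setting Ammo for Throwable.
; It then clears the type and hides the Sphere, leaving collision untouched, and rerolls and reappears after a delay.
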(event Custom|PowerupReset
  (Variables|Default|Setpowerup "")
  (Rendering|SetVisibility (Variables|Default|GetSphere) false true)
  (Utilities|FlowControl|Delay 1e+01)
  (CallFunction|RandomPowerup)
  (Rendering|SetVisibility (Variables|Default|GetSphere) true true))

(event Custom|RandomPowerup
  (bind _staticmesh (Variables|Default|GetStaticMesh))
  (switch int (Math|Random|RandomIntegerinRange 0 2)
    (:0
      (Variables|Default|Setpowerup "Boost")
      (Components|StaticMesh|SetStaticMesh _staticmesh "/Game/Assets/Powerups/redbull/Red_bull_Obee.Red_bull_Obee"))
    (:1
      (Variables|Default|Setpowerup "Throwable")
      (if (> (Math|Random|RandomFloat) 0.5)
        (Components|StaticMesh|SetStaticMesh _staticmesh "/Game/Assets/Powerups/Shortcake/strawberry_short_cake_default.strawberry_short_cake_default")
        (else
          (Components|StaticMesh|SetStaticMesh _staticmesh "/Game/Assets/Powerups/Toast/toast_pCube1.toast_pCube1"))))
    (:2
      (Variables|Default|Setpowerup "MegaTakeDown")
      (Components|StaticMesh|SetStaticMesh _staticmesh "/Game/Assets/Powerups/Burger/burgerunwrapped.burgerunwrapped"))))

(event EventBeginPlay
  (CallFunction|RandomPowerup))

(event Collision|EventActorBeginOverlap
  (params (OtherActor :type Actor%20Object%20Reference))
  (bind _asbp_bike (Utilities|Casting|CastTobp_bike OtherActor))
  (bind _output_get (Variables|/Game/Blueprints/Bike_BP/bp_bike.bp_bike_C|Setpowerup _asbp_bike (Variables|Default|Getpowerup)))
  (if (Utilities|Enum|Equal(Enum) _output_get "Throwable")
    (Variables|/Game/Blueprints/Bike_BP/bp_bike.bp_bike_C|Setammo _asbp_bike 3))
  (CallFunction|PowerupReset))

(fn ConstructionScript)