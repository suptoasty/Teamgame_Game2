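; Stomper is an actor that moves itself vertically along a timeline, starting after a configurable delay from BeginPlay.
; It caches its location once the delay ends, then the MoveBlock timeline adds its ZPosition track to that height without sweeping, keeping X and Y fixed.
; A target position slightly below the start is also stored but does not drive the movement.
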(event EventBeginPlay
  (bind _returnvalue (Transformation|GetActorLocation))
  (bind _originalposition (Variables|Default|GetOriginalPosition))
  (bind (_x _y _z) (Math|Vector|BreakVector _originalposition))
  (bind (_x_2 _y_2 _z_2) (Math|Vector|BreakVector _returnvalue))
  (Utilities|FlowControl|Delay (Variables|Default|Getdelay))
  (bind _output_get (Variables|Default|SetoriginalPosition _returnvalue))
  (bind _output_get_2 (Variables|Default|SettargetPosition (Math|Vector|MakeVector _x_2 _y_2 (- _z_2 1e+01))))
  (bind _z_position (Timeline|MoveBlock Play)
    (:Update
      (Transformation|SetActorLocation (Math|Vector|MakeVector _x _y (+ (.Z (Math|Vector|BreakVector _z_position)) _z)) false false))))

(fn ConstructionScript)