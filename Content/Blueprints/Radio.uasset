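; Radio actor that plays a playlist of songs and lets the player skip forward or back with the NextSong and PrevSong inputs.
; On BeginPlay it enables input, starts the first song on its Audio component and adds a RadioUI widget to the viewport.
; Each skip finds the current sound in the Songs array, wraps to the neighboring track, then briefly shows its asset name on the widget.
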(event EventBeginPlay
  (Input|EnableInput (Game|GetPlayerController 0))
  (CallFunction|PlaySong (Utilities|Array|Get(acopy) (Variables|Default|GetSongs)))
  (bind _returnvalue (UserInterface|CreateWidget "/Game/Widgets/RadioUI.RadioUI_C" (Game|GetPlayerController 0)))
  (bind _output_get (Variables|Default|SetRadioUI _returnvalue))
  (UserInterface|Viewport|AddtoViewport _output_get 0))

(event Collision|EventActorBeginOverlap
  (params (OtherActor :type Actor%20Object%20Reference)))

(event EventTick
  (params (DeltaSeconds :type Float%20%28single-precision%29)))

(event Input|ActionEvents|InputActionNextSong
  (params (Key :type Key%20Structure))
  (bind _radioui (Variables|Default|GetRadioUI))
  (:Pressed
    (bind _newsong (CallFunction|GetNextSong))
    (bind _songname (CallFunction|PlaySong _newsong))
    (Variables|/Game/Widgets/RadioUI.RadioUI_C|SetKickerString _radioui (Utilities|Text|ToText(String) (Utilities|String|Append (Variables|Default|GetKickerString) _songname)))
    (Widget|SetVisibility _radioui "Visible")
    (Utilities|FlowControl|Delay 0.5)
    (Widget|SetVisibility _radioui "Hidden")))

(event Input|ActionEvents|InputActionPrevSong
  (params (Key :type Key%20Structure))
  (bind _radioui (Variables|Default|GetRadioUI))
  (:Pressed
    (bind _newsong (CallFunction|GetPrevSong))
    (bind _songname (CallFunction|PlaySong _newsong))
    (Variables|/Game/Widgets/RadioUI.RadioUI_C|SetKickerString _radioui (Utilities|Text|ToText(String) (Utilities|String|Append (Variables|Default|GetKickerString) _songname)))
    (Widget|SetVisibility _radioui "Visible")
    (Utilities|FlowControl|Delay 0.5)
    (Widget|SetVisibility _radioui "Hidden")))

(fn ConstructionScript)

(fn PlaySong
  (params (NewParam :type Sound%20Wave%20Object%20Reference))
  (bind _audio (Variables|Default|GetAudio))
  (Audio|Components|Audio|SetSound _audio NewParam)
  (Audio|Components|Audio|Play _audio 0.0)
  (return (Utilities|GetObjectName (Variables|/Script/Engine.AudioComponent|GetSound _audio))))

(fn GetNextSong
  (bind _songs (Variables|Default|GetSongs))
  (for (_array_element _array_index) _songs
    (if (== _array_element (Variables|/Script/Engine.AudioComponent|GetSound (Variables|Default|GetAudio)))
      (return (Utilities|Array|Get(acopy) _songs (Math|Integer|%(Integer) (+ _array_index 1) (Utilities|Array|Length _songs)))))))

(fn GetPrevSong
  (bind _songs (Variables|Default|GetSongs))
  (bind _returnvalue (Utilities|Array|Length _songs))
  (for (_array_element _array_index) _songs
    (if (== _array_element (Variables|/Script/Engine.AudioComponent|GetSound (Variables|Default|GetAudio)))
      (if (< (- _array_index 1) 0)
        (return (Utilities|Array|Get(acopy) _songs (- _returnvalue 1)))
        (else
          (return (Utilities|Array|Get(acopy) _songs (Math|Integer|%(Integer) (- _array_index 1) _returnvalue))))))))