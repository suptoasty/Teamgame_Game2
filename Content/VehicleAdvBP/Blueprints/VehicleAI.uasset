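; VehicleAI is a path-following helper that steers a referenced vehicle along the Path spline.
; Each Tick it offsets the vehicle's position 500 units against the spline's nearest local right vector, used as travel direction, to look ahead.
; The spline point closest to that position becomes the vehicle's Steering target.
; A Sphere shows the target, and a yaw-flipped Arrow marks the vehicle's nearest point on the curve.
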(event EventTick
  (params (DeltaSeconds :type Float%20%28single-precision%29))
  (bind _path (Variables|Default|GetPath))
  (bind _path_2 (Variables|Default|GetPath))
  (bind _vehiclereff (Variables|Default|GetVehicleReff))
  (bind _returnvalue (Transformation|GetActorLocation _vehiclereff))
  (bind _returnvalue_2 (Class|SplineComponent|FindRightVectorClosesttoWorldLocation _path_2 _returnvalue "Local"))
  (bind _returnvalue_3 (Math|Rotator|MakeRotationfromAxes _returnvalue_2 "0, 0, 0" "0, 0, 0"))
  (bind (_roll _pitch _yaw) (Math|Rotator|BreakRotator _returnvalue_3))
  (bind _output_get (Variables|/Game/VehicleAdvBP/Blueprints/VehicleBlueprint.VehicleBlueprint_C|SetSteering (Variables|Default|GetVehicleReff) (Spline|FindLocationClosesttoWorldLocation _path (- _returnvalue (* (Math|Vector|GetForwardVector _returnvalue_3) 500)) "World")))
  ;[1 1 1] Display point being turned towards
  (Transformation|SetWorldLocation (Variables|Default|GetSphere) _output_get false false)
  ;[1 1 1] Display position on curve
  (Transformation|SetWorldLocationAndRotation (Variables|Default|GetArrow) (Spline|FindLocationClosesttoWorldLocation _path _returnvalue "World") (Math|Rotator|MakeRotator _roll _pitch (- _yaw 1.8e+02)) false false))

(fn ConstructionScript)